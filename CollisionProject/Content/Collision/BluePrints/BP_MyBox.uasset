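; BP_MyBox is a trigger box Blueprint that starts motion when something overlaps its Cube2 component.
; The overlap event loops over the MoveRect array and plays each element, also calling Play on RotationBall and MoveLeftRight on every iteration.
; It does not filter which actor overlaps.
; BeginPlay and the construction script are empty, and a leftover Sequence of loops printing indices is never executed.
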(event OnComponentBeginOverlap(Cube2)
  (params (OverlappedComponent :type Primitive%20Component%20Object%20Reference) (OtherActor :type Actor%20Object%20Reference) (OtherComp :type Primitive%20Component%20Object%20Reference) (OtherBodyIndex :type Integer) (bFromSweep :type Boolean) (SweepResult :type Hit%20Result%20Structure%20%28by%20ref%29))
  (for _array_element (Variables|Default|GetMoveRect)
    (Default|Play _array_element)
    (Default|Play (Variables|Default|GetRotationBall))
    (Default|Play (Variables|Default|GetMoveLeftRight))))

(event EventBeginPlay)

(fn ConstructionScript)